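; Player character Blueprint for a 2D side-view fighter, with limited multi-jump, ammo-limited shooting, a blink teleport and a cooldown-gated summon.
; Input, landing and damage events set the Stanje state, which UpdateAnimation maps to flipbooks every Tick.
; Tick also sets facing, blink offset and edge-aware sweeping, and toggles a collision channel for jumping up or dropping through platforms.
; Damage handlers reduce health, disable input on death, and apply knockback from player 1's character for melee.
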(event `InputAction|Jump`
  (params (Key :type "Key Structure" :default "AnyKey"))
  (bind _brojskokova (`self.brojskokova`))
  ;[1 1 1] kontrola skakanja
  (:`Pressed`
    (if (< _brojskokova (`self.maxskokova`))
      (bind _output_get (set `self.brojskokova` (+ _brojskokova 1)))
      (if (>= _output_get 2)
        (`self.Jump`)
        (set `self.stanje` "NewEnumerator2")
        (else
          (`self.Jump`)
          (set `self.stanje` "NewEnumerator2")))
      (`self.prasina_skok`)))
  (:`Released`
    (`self.StopJumping` :!label _label)))

(event `InputTouch`
  (params (Location :type "Vector Structure") (FingerIndex :type "ETouchIndex Enum"))
  ;[1 1 1] kontrola skakanja
  (:`Released`
    (goto _label)))

(event `self.ReceiveBeginPlay`
  ;[1 1 1] hud i inicjalizacija!!!!
  (set `PlayerController.bShowMouseCursor` true (`GameplayStatics.GetPlayerController` 0))
  (`WidgetLayoutLibrary.RemoveAllWidgets`)
  (`|ExecutionSequence`
    (:`then_0`
      (`ActorComponent.SetIsReplicated` (`self.Sprite`) true))
    (:`then_1`
      (bind _returnvalue (`|CreateWidget` "/Game/purgatorium/bluprint/Hud.Hud_C" (`GameplayStatics.GetPlayerController` 0)))
      (bind _output_get (set `self.heltbar` _returnvalue))
      (`UserWidget.AddToViewport` _output_get 0))))

(event `self.ReceiveActorBeginOverlap`
  (params (OtherActor :type "Actor Object Reference"))
  ;[1 1 1] kolizjoni filter
  ;;[0 1 0.04817] filter za skok
  (`|ExecutionSequence`
    (:`then_0`
      (cast `/Game/purgatorium/bluprint/kolajder` OtherActor))
    (:`then_1`
      (cast `/Game/purgatorium/bluprint/kolajder_zanovilvl` OtherActor)))
  (set `self.cekkolajdera` true))

(event `self.ReceiveActorEndOverlap`
  (params (OtherActor :type "Actor Object Reference"))
  ;[1 1 1] kolizjoni filter
  ;;[0 1 0.04817] filter za skok
  (`|ExecutionSequence`
    (:`then_0`
      (cast `/Game/purgatorium/bluprint/kolajder` OtherActor))
    (:`then_1`
      (cast `/Game/purgatorium/bluprint/kolajder_zanovilvl` OtherActor)))
  (set `self.cekkolajdera` false))

(event `self.OnLanded`
  (params (Hit :type "HitResult Structure (by ref)"))
  ;[1 1 1] kontrola skakanja
  (if (<= (`self.helt`) 0.0)
    (set `self.stanje` "NewEnumerator5")
    (set `self.brojskokova` 0)
    (else
      (set `self.stanje` "NewEnumerator0")
      (set `self.brojskokova` 0)
      (`self.prasina_sletanje`))))

(event `self.OnJumped`
  ;[1 1 1] kolizjoni filter
  ;;[0 1 0.04817] filter za skok
  (set `self.cekskok` true)
  (`PrimitiveComponent.SetCollisionResponseToChannel` (`self.CapsuleComponent`) "ECC_GameTraceChannel1" "ECR_Overlap"))

(event `self.ReceiveTick`
  (params (DeltaSeconds :type "Float (single-precision)"))
  (bind (_returnvalue_x _returnvalue_y _returnvalue_z) (`KismetMathLibrary.BreakVector` (`self.GetVelocity`)))
  (bind _returnvalue_x_2 (`KismetMathLibrary.BreakVector` (`SceneComponent.K2_GetComponentLocation` (`self.CapsuleComponent`))))
  (bind _returnvalue_x_3 (`KismetMathLibrary.BreakVector` (`SceneComponent.K2_GetComponentLocation` (`self.CapsuleComponent`))))
  ;[1 1 1] kontrola kretanja
  (`self.UpdateAnimation`)
  (`|ExecutionSequence`
    (:`then_0`
      ;;[0 1 0.04817] udaljenost blinka!!!
      (`/Engine/EditorBlueprintResources/StandardMacros.CompareInt` (`self.pravac`) 1
        (:`==`
          (set `self.vektor_za_teleport` (-700.0 0.0 0.0)))
        (:`<`
          (set `self.vektor_za_teleport` (700.0 0.0 0.0))))
      (`/Engine/EditorBlueprintResources/StandardMacros.CompareFloat` (.x (`MovementComponent.Velocity` (`self.GetMovementComponent`)))
        (:`>`
          (`Controller.SetControlRotation` (`self.GetController`) (`KismetMathLibrary.MakeRotator` 0.0 0.0 0.0) :!label _label_2)
          (set `self.pravac` -1))
        (:`==`
          (if (`self.bisMovingRight`)
            (goto _label_2)
            (else
              (`Controller.SetControlRotation` (`self.GetController`) (`KismetMathLibrary.MakeRotator` 0.0 0.0 180.0) :!label _label_3)
              (set `self.pravac` 1))))
        (:`<`
          (goto _label_3)))
      (`|ExecutionSequence`
        (:`then_0`
          ;[1 1 1] kolizjoni filter
          ;;[0 1 0.04817] filter za skok
          (if (< _returnvalue_z 0.0)
            (set `self.cekpadanja` true)
            (set `self.cekskok` false)
            (if (not (`self.cekkolajdera`))
              (`PrimitiveComponent.SetCollisionResponseToChannel` (`self.CapsuleComponent`) "ECC_GameTraceChannel1" "ECR_Block"))
            (else
              (set `self.cekpadanja` false))))
        (:`then_1`
          ;;[0 1 0.04817] filter za propadanje!
          (if (`self.pritisnuto`)
            (`PrimitiveComponent.SetCollisionResponseToChannel` (`self.CapsuleComponent`) "ECC_GameTraceChannel1" "ECR_Overlap")))))
    (:`then_1`
      ;[1 1 1] kontrola_pravca za teleport
      (`/Engine/EditorBlueprintResources/StandardMacros.CompareFloat` _returnvalue_x_2 3200.0
        (:`>`
          (set `self.teleport` false)
          (set `self.svip` true))
        (:`<`
          (set `self.teleport` true)
          (set `self.svip` false))))
    (:`then_2`
      (`/Engine/EditorBlueprintResources/StandardMacros.CompareFloat` _returnvalue_x_3 -2200.0
        (:`<`
          (set `self.teleport` false)
          (set `self.svip` true))))))

(event `InputAxis|MoveRight`
  (params (AxisValue :type "Float (single-precision)"))
  ;[1 1 1] kontrola kretanja
  (`|ExecutionSequence`
    (:`then_0`
      (if (`self.cekKretanja`)
        (if (> AxisValue 0.0)
          (set `self.bisMovingRight` true)
          (elif (< AxisValue 0.0)
            (set `self.bisMovingRight` false)))
        (`self.AddMovementInput` (1.0 0.0 0.0) AxisValue)))))

(event `InputAction|dolje`
  (params (Key :type "Key Structure" :default "AnyKey"))
  ;[1 1 1] kolizjoni filter
  ;;[0 1 0.04817] filter za propadanje!
  (:`Pressed`
    (set `self.pritisnuto` true)
    (`CharacterMovementComponent.AddForce` (`self.CharacterMovement`) (0.0 0.0 -3000000.0)))
  (:`Released`
    (set `self.pritisnuto` false)))

(event `self.OnWalkingOffLedge`
  (params (PreviousFloorImpactNormal :type "Vector Structure (by ref)") (PreviousFloorContactNormal :type "Vector Structure (by ref)") (PreviousLocation :type "Vector Structure (by ref)") (TimeDelta :type "Float (single-precision)"))
  ;[1 1 1] pad sa kolajdera
  (set `self.stanje` "NewEnumerator2"))

(event `InputAction|pucanj`
  (params (Key :type "Key Structure" :default "AnyKey"))
  (bind _broj_metaka (`self.broj_metaka`))
  ;[1 1 1] pucanje
  (:`Pressed`
    (set `self.broj_metaka` (- _broj_metaka 1))
    (if (<= _broj_metaka 0)
      (`KismetSystemLibrary.Delay` 2.0)
      (set `self.broj_metaka` 6)
      (else
        (bind _returnvalue (`|SpawnActorFromClass` "/Game/purgatorium/bluprint/bp_zrno.bp_zrno_C" (`SceneComponent.K2_GetComponentToWorld` (`self.Arrow1`)) "AlwaysSpawn" "OverrideRootScale"))
        (bind _returnvalue_2 (`|SpawnActorFromClass` "/Game/purgatorium/bluprint/bp_zrno.bp_zrno_C" (`SceneComponent.K2_GetComponentToWorld` (`self.Arrow5`)) "AlwaysSpawn" "OverrideRootScale"))
        (set `self.stanje` "NewEnumerator6")
        (`MovementComponent.StopMovementImmediately` (`self.CharacterMovement`))
        (`KismetSystemLibrary.RetriggerableDelay` 0.4)
        (set `self.stanje` "NewEnumerator0")
        (`self.UpdateAnimation`)
        (`self.SetLifeSpan` _returnvalue 20.0)
        (`self.SetLifeSpan` _returnvalue_2 20.0)))))

(event `UpdateAnimation`
  ;[1 1 1] kontrola animacije
  (switch `/Game/purgatorium/bluprint/stanja` (`self.stanje`)
    (:`NewEnumerator0`
      (`PaperFlipbookComponent.SetFlipbook` (`self.Sprite`) (select `bool` (> (`KismetMathLibrary.VSize` (`self.GetVelocity`)) 0.0) :`false` "/Game/purgatorium/sprajtovi/Art/karakter/disanje/disanje.disanje" :`true` "/Game/purgatorium/sprajtovi/Art/karakter/trcanje.trcanje" :!type "PaperFlipbook Object Reference")))
    (:`NewEnumerator2`
      (`PaperFlipbookComponent.SetFlipbook` (`self.Sprite`) "/Game/purgatorium/sprajtovi/Art/karakter/skokanime.skokanime"))
    (:`NewEnumerator3`
      (`PaperFlipbookComponent.SetFlipbook` (`self.Sprite`) "/Game/purgatorium/sprajtovi/Art/cucanj/karakter_-_cucanj2_export.karakter_-_cucanj2_export"))
    (:`NewEnumerator4`
      (`PaperFlipbookComponent.SetFlipbook` (`self.Sprite`) "/Game/purgatorium/sprajtovi/Art/pucanje/karakter_-_damage.karakter_-_damage"))
    (:`NewEnumerator5`
      (`PaperFlipbookComponent.SetFlipbook` (`self.Sprite`) "/Game/purgatorium/sprajtovi/Art/karakter/umiranjeD.umiranjeD"))
    (:`NewEnumerator6`
      (`PaperFlipbookComponent.SetFlipbook` (`self.Sprite`) "/Game/purgatorium/sprajtovi/Art/pucanje/PUCANJE.PUCANJE"))
    (:`NewEnumerator7`
      (`PaperFlipbookComponent.SetFlipbook` (`self.Sprite`) "/Game/purgatorium/sprajtovi/Art/karakter/disanje/disanje.disanje"))
    (:`NewEnumerator9`
      (`PaperFlipbookComponent.SetFlipbook` (`self.Sprite`) "/Game/purgatorium/sprajtovi/Art/udarac_sakom/karakter_-_punch.karakter_-_punch"))
    (:`NewEnumerator10`
      (`PaperFlipbookComponent.SetFlipbook` (`self.Sprite`) "/Game/purgatorium/sprajtovi/Art/aperkat/karakter_-_skok_dupli.karakter_-_skok_dupli"))
    (:`NewEnumerator11`
      (`PaperFlipbookComponent.SetFlipbook` (`self.Sprite`) "/Game/purgatorium/sprajtovi/Art/prizivanje/karakter_-_summon_export.karakter_-_summon_export"))
    (:`NewEnumerator12`
      (`PaperFlipbookComponent.SetFlipbook` (`self.Sprite`) "/Game/purgatorium/sprajtovi/Art/pucanje_nagore/karakter_-_pucanje_gore.karakter_-_pucanje_gore"))
    (:`NewEnumerator13`
      (`PaperFlipbookComponent.SetFlipbook` (`self.Sprite`) "/Game/purgatorium/sprajtovi/Art/teleport/karakter_-_TELEPORT_ulaz.karakter_-_TELEPORT_ulaz"))
    (:`NewEnumerator14`
      (`PaperFlipbookComponent.SetFlipbook` (`self.Sprite`) "/Game/purgatorium/sprajtovi/Art/teleport/karakter_-_TELEPORT_izlaz.karakter_-_TELEPORT_izlaz"))))

(event `prasina_sletanje`
  ;[1 0 0] EFEKTI!!!!!
  ;;[1 1 1] prasina_sletanje
  (bind _returnvalue (`|SpawnActorFromClass` "/Game/purgatorium/bluprint/props/bp_sletanje.bp_sletanje_C" (`SceneComponent.K2_GetComponentToWorld` (`self.Arrow2`)) "AlwaysSpawn" "OverrideRootScale"))
  (`self.SetLifeSpan` _returnvalue 1.0))

(event `prasina_trcanje`
  ;[1 0 0] EFEKTI!!!!!
  ;;[1 1 1] prasina_trcanje
  (bind _returnvalue (`|SpawnActorFromClass` "/Game/purgatorium/bluprint/props/bp_sletanje.bp_sletanje_C" (`SceneComponent.K2_GetComponentToWorld` (`self.Arrow2`)) "AlwaysSpawn" "OverrideRootScale"))
  (`self.SetLifeSpan` _returnvalue 1.0))

(event `prasina_skok`
  ;[1 0 0] EFEKTI!!!!!
  ;;[1 1 1] prasina_skok
  (bind _returnvalue (`|SpawnActorFromClass` "/Game/purgatorium/bluprint/props/bp_prasina_skok.bp_prasina_skok_C" (`SceneComponent.K2_GetComponentToWorld` (`self.Arrow2`)) "AlwaysSpawn" "OverrideRootScale"))
  (`self.SetLifeSpan` _returnvalue 0.5))

(event `InputAction|blink`
  (params (Key :type "Key Structure" :default "AnyKey"))
  (bind _capsulecomponent (`self.CapsuleComponent`))
  ;[1 1 1] blink
  (:`Pressed`
    (if (not (`self.DaLiTeleport`))
      (set `self.DaLiTeleport` true)
      (set `self.stanje` "NewEnumerator13")
      (`KismetSystemLibrary.Delay` 0.2)
      (`SceneComponent.K2_SetWorldLocation` _capsulecomponent (+ (`SceneComponent.K2_GetComponentLocation` _capsulecomponent) (`self.vektor_za_teleport`)) (`self.svip`) (`self.teleport`))
      (set `self.stanje` "NewEnumerator14")
      (`KismetSystemLibrary.Delay` 0.2)
      (set `self.stanje` "NewEnumerator0")
      (`KismetSystemLibrary.Delay` 0.2)))
  (:`Released`
    (`KismetSystemLibrary.Delay` 1.0)
    (set `self.DaLiTeleport` false)))

(event `InputAction|pucanje po zedu`
  (params (Key :type "Key Structure" :default "AnyKey"))
  ;[1 1 1] pucanje po zedu
  (:`Pressed`
    (if (not (`self.DaLiSamon`))
      (set `self.DaLiSamon` true)
      (`self.DisableInput` null)
      (set `self.stanje` "NewEnumerator11")
      (`KismetSystemLibrary.Delay` 0.4)
      (`self.EnableInput` null)
      (set `self.stanje` "NewEnumerator0")
      (bind _returnvalue (`|SpawnActorFromClass` "/Game/purgatorium/bluprint/Kain_Usijane_Glave.Kain_Usijane_Glave_C" (`SceneComponent.K2_GetComponentToWorld` (`self.Arrow6`)) "AlwaysSpawn" "OverrideRootScale"))
      (bind _returnvalue_2 (`|SpawnActorFromClass` "/Game/purgatorium/bluprint/Kain_Usijane_GlaveZ.Kain_Usijane_GlaveZ_C" (`SceneComponent.K2_GetComponentToWorld` (`self.Arrow6`)) "AlwaysSpawn" "OverrideRootScale"))
      (bind _returnvalue_3 (`|SpawnActorFromClass` "/Game/purgatorium/bluprint/Mitropolit_Usijane_GlaveX.Mitropolit_Usijane_GlaveX_C" (`SceneComponent.K2_GetComponentToWorld` (`self.Arrow6`)) "AlwaysSpawn" "OverrideRootScale"))
      (`self.SetLifeSpan` _returnvalue 5.0)
      (`self.SetLifeSpan` _returnvalue_2 5.0)
      (`self.SetLifeSpan` _returnvalue_3 5.0)))
  (:`Released`
    (`KismetSystemLibrary.Delay` (`self.allKULL`))
    (set `self.DaLiSamon` false)))

(event `dmg sistem`
  (params (dmgin :type "Float (double-precision)"))
  ;[1 1 1] dmg sistem
  (set `self.cekDMG` true)
  (bind _output_get (set `self.helt` (- (`self.helt`) dmgin)))
  (if (<= _output_get 0.0)
    (set `self.stanje` "NewEnumerator5")
    (`|ExecutionSequence`
      (:`then_0`
        (`self.DisableInput` (`GameplayStatics.GetPlayerController` 0)))
      (:`then_1`
        (`self.DisableInput` (`GameplayStatics.GetPlayerController` 1))))
    (else
      (set `self.stanje` "NewEnumerator4")
      (`CharacterMovementComponent.AddForce` (`self.CharacterMovement`) (0.0 0.0 800000.0)))))

(event `DMG_sistem_mele`
  (params (dmgin :type "Float (double-precision)"))
  ;[1 1 1] dmg sistem mele
  (set `self.cekDMG` true)
  (bind _output_get (set `self.helt` (- (`self.helt`) dmgin)))
  (if (<= _output_get 0.0)
    (set `self.stanje` "NewEnumerator5")
    (`|ExecutionSequence`
      (:`then_0`
        (`self.DisableInput` (`GameplayStatics.GetPlayerController` 0)))
      (:`then_1`
        (`self.DisableInput` (`GameplayStatics.GetPlayerController` 1))))
    (else
      (set `self.stanje` "NewEnumerator4")
      (`|ExecutionSequence`
        (:`then_0`
          (bind _asbp_kain_sake (cast `/Game/purgatorium/bluprint/bp_kainSake` (`GameplayStatics.GetPlayerCharacter` 1)))
          (`self.LaunchCharacter` (`KismetMathLibrary.MakeVector` (* (`/Game/purgatorium/bluprint/bp_kainSake.pravac` _asbp_kain_sake) (`self.udar`)) 0.0 0.0) true true))
        (:`then_1`
          (bind _asbp_kain (cast `/Game/purgatorium/bluprint/bp_kain` (`GameplayStatics.GetPlayerCharacter` 1)))
          (`self.LaunchCharacter` (`KismetMathLibrary.MakeVector` (* (`/Game/purgatorium/bluprint/bp_kain.pravac` _asbp_kain) (`self.udar`)) 0.0 0.0) true true))))))

(fn `UserConstructionScript`)